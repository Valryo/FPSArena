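; A health pickup that fully heals a Player overlapping its static mesh, unless that player is already at full health.
; On pickup it hides the mesh, disables its collision and plays a sound.
; A timer then calls SetVisible after RespawnTime to restore visibility and collision, so the same actor respawns without being destroyed.
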(event `self.StaticMesh.OnComponentBeginOverlap`
  (params (OverlappedComponent :type "PrimitiveComponent Object Reference") (OtherActor :type "Actor Object Reference") (OtherComp :type "PrimitiveComponent Object Reference") (OtherBodyIndex :type Integer) (bFromSweep :type Boolean) (SweepResult :type "HitResult Structure (by ref)"))
  (bind _staticmesh (`self.StaticMesh`))
  (bind _asplayer (cast `/Game/Player/Player` OtherActor))
  (bind _fullhealth (`/Game/Player/Player.IsFullHealth` _asplayer))
  (if (not _fullhealth)
    (`/Game/Player/Player.SetToFullHealth` _asplayer)
    (`SceneComponent.SetVisibility` _staticmesh false true)
    (`PrimitiveComponent.SetCollisionEnabled` _staticmesh "NoCollision")
    (`AudioComponent.Play` (`self.Audio`) 0.0)
    (`KismetSystemLibrary.K2_SetTimer` self "SetVisible" (`self.RespawnTime`))))

(fn `SetVisible`
  (bind _staticmesh (`self.StaticMesh`))
  (`SceneComponent.SetVisibility` _staticmesh true true)
  (`PrimitiveComponent.SetCollisionEnabled` _staticmesh "QueryAndPhysics"))

(fn `UserConstructionScript`)