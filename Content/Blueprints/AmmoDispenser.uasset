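; Ammo dispenser actor that refills a player's weapons while they stand inside its AmmoSphere trigger.
; On overlap begin with a Player, it starts looping one-second timers that call AddAmmo by name on the primary and secondary weapons.
; On overlap end it clears those timers, so the refill logic lives in the weapons themselves.
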(event `self.AmmoSphere.OnComponentBeginOverlap`
  (params (OverlappedComponent :type "PrimitiveComponent Object Reference") (OtherActor :type "Actor Object Reference") (OtherComp :type "PrimitiveComponent Object Reference") (OtherBodyIndex :type Integer) (bFromSweep :type Boolean) (SweepResult :type "HitResult Structure (by ref)"))
  (bind _asplayer (cast `/Game/Player/Player` OtherActor))
  (`KismetSystemLibrary.K2_SetTimer` (`/Game/Player/Player.PrimaryWeapon` _asplayer) "AddAmmo" 1.0 true)
  (`KismetSystemLibrary.K2_SetTimer` (`/Game/Player/Player.SecondaryWeapon` _asplayer) "AddAmmo" 1.0 true))

(event `self.AmmoSphere.OnComponentEndOverlap`
  (params (OverlappedComponent :type "PrimitiveComponent Object Reference") (OtherActor :type "Actor Object Reference") (OtherComp :type "PrimitiveComponent Object Reference") (OtherBodyIndex :type Integer))
  (bind _asplayer (cast `/Game/Player/Player` OtherActor))
  (`KismetSystemLibrary.K2_ClearTimer` (`/Game/Player/Player.PrimaryWeapon` _asplayer) "AddAmmo")
  (`KismetSystemLibrary.K2_ClearTimer` (`/Game/Player/Player.SecondaryWeapon` _asplayer) "AddAmmo"))

(fn `UserConstructionScript`)