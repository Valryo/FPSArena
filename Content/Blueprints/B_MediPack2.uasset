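; B_MediPack2 is a health pickup that restores a Player to full health.
; On BeginPlay it adds itself to the DeathMatch game mode's HealthPickUps list.
; When a Player begins overlapping its StaticMesh and is below full health, it calls SetToFullHealth on that player, then UsePickUp.
; Players already at full health do not consume it.
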(event `self.ReceiveBeginPlay`
  (bind _asdeath_match (cast `/Game/Blueprints/DeathMatch` (`GameplayStatics.GetGameMode`)))
  (`KismetArrayLibrary.Array_AddUnique` (`/Game/Blueprints/DeathMatch.HealthPickUps` _asdeath_match) self))

(event `self.StaticMesh.OnComponentBeginOverlap`
  (params (OverlappedComponent :type "PrimitiveComponent Object Reference") (OtherActor :type "Actor Object Reference") (OtherComp :type "PrimitiveComponent Object Reference") (OtherBodyIndex :type Integer) (bFromSweep :type Boolean) (SweepResult :type "HitResult Structure (by ref)"))
  (bind _asplayer (cast `/Game/Player/Player` OtherActor))
  (bind _fullhealth (`/Game/Player/Player.IsFullHealth` _asplayer))
  (if (not _fullhealth)
    (`/Game/Player/Player.SetToFullHealth` _asplayer)
    (`self.UsePickUp`)))

(fn `UserConstructionScript`
  (`parent.UserConstructionScript`))