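; Base pickup Blueprint that hides itself when used and respawns after a delay.
; UsePickUp deactivates it, hides the static mesh, disables its collision and plays a sound.
; A timer set to RespawnTime then calls SetVisible by name, restoring visibility, collision and the IsActive flag.
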(fn `SetVisible`
  (bind _staticmesh (`self.StaticMesh`))
  (`SceneComponent.SetVisibility` _staticmesh true true)
  (`PrimitiveComponent.SetCollisionEnabled` _staticmesh "QueryAndPhysics")
  (set `self.isActive` true))

(fn `UsePickUp`
  (bind _staticmesh (`self.StaticMesh`))
  (set `self.isActive` false)
  (`SceneComponent.SetVisibility` _staticmesh false true)
  (`PrimitiveComponent.SetCollisionEnabled` _staticmesh "NoCollision")
  (`AudioComponent.Play` (`self.Audio`) 0.0)
  (`KismetSystemLibrary.K2_SetTimer` self "SetVisible" (`self.RespawnTime`)))

(fn `UserConstructionScript`)