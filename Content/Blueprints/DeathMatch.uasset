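; Deathmatch game mode for an FPS with players and AI bots, running timed rounds scored by kills.
; A one-second timer copies the countdown to every FPSState; at zero EndGame flags top scorers, then Reset restarts after a delay.
; KilledCharacter credits killers or penalizes killerless deaths, and server-side Respawn possesses new pawns at random PlayerStarts.
; PostLogin numbers player names; BeginPlay's bot-spawn loop has an empty range (1 to 0).
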(event `Decount`
  (bind _time (`self.Time`))
  (if (not (== _time 0))
    (bind _result (`/Engine/EditorBlueprintResources/StandardMacros.DecrementInt` _time)
      (:`  `
        (bind _outactors (`GameplayStatics.GetAllActorsOfClass` "/Game/Player/FPSState.FPSState_C"))
        (for _array_element _outactors
          (bind _output_get (set `/Game/Player/FPSState.currentTime` _result _array_element))
          (if (== _output_get 0)
            (`self.EndGame`)))))))

(event `self.ReceiveBeginPlay`
  (`|ExecutionSequence`
    (:`then_0`
      (`KismetSystemLibrary.K2_SetTimerDelegate` (delegate `Decount`) 1.0 true))
    (:`then_1`
      (for _ (range 1 1)
        (bind _transform (`self.RandomStart`))
        (bind _returnvalue (`|SpawnActorFromClass` "/Game/AI/BotPawn.BotPawn_C" _transform "AdjustIfPossibleButAlwaysSpawn" "OverrideRootScale"))
        (`Pawn.SpawnDefaultController` (`Actor.Instigator` _returnvalue))))))

(event `Respawn`
  (params (controller :type "Controller Object Reference"))
  (bind _outactors (`GameplayStatics.GetAllActorsOfClass` "/Script/Engine.PlayerStart"))
  (`/Engine/EditorBlueprintResources/StandardMacros.IsValid` controller
    (:`Is Valid`
      (`/Engine/EditorBlueprintResources/ActorMacros.Switch Has Authority`
        (:`Authority`
          (bind _asshooter_aicontroller (cast `/Game/AI/ShooterAIController` controller)
            (:`then`
              (bind _returnvalue (`self.GetTransform` (`KismetArrayLibrary.Array_Get` _outactors (`KismetMathLibrary.RandomInteger` (`KismetArrayLibrary.Array_Length` _outactors)))))
              (bind _returnvalue_2 (`|SpawnActorFromClass` "/Game/AI/BotPawn.BotPawn_C" _returnvalue "AdjustIfPossibleButAlwaysSpawn" "OverrideRootScale"))
              (`Controller.Possess` _asshooter_aicontroller _returnvalue_2)
              (`/Game/AI/ShooterAIController.Respawn` _asshooter_aicontroller))
            (:`CastFailed`
              (bind _returnvalue_3 (`|SpawnActorFromClass` "/Game/Player/Player.Player_C" _returnvalue "AdjustIfPossibleButAlwaysSpawn" "OverrideRootScale"))
              (`Controller.Possess` controller _returnvalue_3))))))))

(event `self.K2_PostLogin`
  (params (NewPlayer :type "PlayerController Object Reference"))
  (bind _numberplayer (`self.NumberPlayer`))
  (bind _asfpsplayer_controller (cast `/Game/Player/FPSPlayerController` NewPlayer))
  (bind _name (`/Game/Player/FPSPlayerController.GetName` _asfpsplayer_controller))
  (`self.ChangeName` NewPlayer (`KismetStringLibrary.BuildString_Int` _name "#" _numberplayer))
  (`/Engine/EditorBlueprintResources/StandardMacros.IncrementInt` _numberplayer))

(fn `EndGame`
  (locals (MaxScore :type Integer))
  (bind _maxscore (`local.MaxScore`))
  (`KismetSystemLibrary.K2_SetTimer` self "Reset" 5.0)
  (bind _outactors (`GameplayStatics.GetAllActorsOfClass` "/Game/Player/FPSState.FPSState_C"))
  (for _array_element _outactors
    (set `local.MaxScore` (`KismetMathLibrary.Max` (`/Game/Player/FPSState.currentScore` _array_element) _maxscore)))
  (for _array_element_2 _outactors
    (`/Game/Player/FPSState.EndGame` _array_element_2 (== _maxscore (`/Game/Player/FPSState.currentScore` _array_element_2)))))

(fn `KilledCharacter`
  (params (killed :type "Controller Object Reference") (Killer :type "Controller Object Reference"))
  (`/Engine/EditorBlueprintResources/StandardMacros.IsValid` Killer
    (:`Is Valid`
      (bind _asfpsstate (cast `/Game/Player/FPSState` (`Controller.PlayerState` Killer)))
      (set `/Game/Player/FPSState.currentScore` (+ (`/Game/Player/FPSState.currentScore` _asfpsstate) 1) _asfpsstate))
    (:`Is Not Valid`
      (`/Engine/EditorBlueprintResources/StandardMacros.IsValid` killed
        (:`Is Valid`
          (bind _asfpsstate_2 (cast `/Game/Player/FPSState` (`Controller.PlayerState` killed)))
          (set `/Game/Player/FPSState.currentScore` (- (`/Game/Player/FPSState.currentScore` _asfpsstate_2) 1) _asfpsstate_2))))))

(fn `RandomStart`
  (returns (Transform :type "Transform Structure"))
  (bind _outactors (`GameplayStatics.GetAllActorsOfClass` "/Script/Engine.PlayerStart"))
  (return (`self.GetTransform` (`KismetArrayLibrary.Array_Get` _outactors (`KismetMathLibrary.RandomInteger` (`KismetArrayLibrary.Array_Length` _outactors))))))

(fn `Reset`
  (`self.ResetLevel`)
  (set `self.Time` (`self.DefaultTime`))
  (bind _outactors (`GameplayStatics.GetAllActorsOfClass` "/Script/Engine.Controller"))
  (for _array_element _outactors
    (`self.Respawn` _array_element))
  (bind _outactors_2 (`GameplayStatics.GetAllActorsOfClass` "/Game/Player/FPSState.FPSState_C"))
  (for _array_element_2 _outactors_2
    (set `/Game/Player/FPSState.currentScore` 0 _array_element_2)
    (set `/Game/Player/FPSState.Message` "" _array_element_2)))

(fn `UserConstructionScript`)