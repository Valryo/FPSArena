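; Team deathmatch game logic that splits players into two teams and declares a winner when the game ends.
; NewPlayer balances joins by team size and stamps the team number on each FPSState, while RemovePlayer clears leavers from both lists.
; On EndGame, it sums kills per team from the PlayerArray, tells every player state the winner (Red takes ties), and schedules Reset after RestartTime.
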(event `self.EndGame`
  (`self.EndGameTeam`))

(fn `EndGameTeam`
  (bind _restarttime (`self.RestartTime`))
  (`KismetSystemLibrary.K2_SetTimer` self "Reset" (`self.RestartTime`))
  (bind (_team1score _team2score) (`self.GetTeamScore`))
  (for _array_element (`GameStateBase.PlayerArray` (`GameplayStatics.GetGameState`))
    (bind _asfpsstate (cast `/Game/Player/FPSState` _array_element))
    (if (> _team1score _team2score)
      (`/Game/Player/FPSState.GameHasEnded` _asfpsstate "Blue team" _restarttime)
      (else
        (`/Game/Player/FPSState.GameHasEnded` _asfpsstate "Red team" _restarttime)))
    (set `self.GameHasEnded` true)))

(fn `GetTeamScore`
  (returns (Team1score :type Integer) (Team2score :type Integer))
  (locals (T1Score :type Integer) (T2Score :type Integer))
  (for _array_element (`GameStateBase.PlayerArray` (`GameplayStatics.GetGameState`))
    (bind _asfpsstate (cast `/Game/Player/FPSState` _array_element))
    (switch `int` (`/Game/Player/FPSState.TeamNumber` _asfpsstate)
      (:`1`
        (bind _nbkills (`/Game/Player/FPSState.NbKills` _asfpsstate))
        (set `local.T1Score` (+ (`local.T1Score`) _nbkills)))
      (:`2`
        (set `local.T2Score` (+ _nbkills (`local.T2Score`))))))
  (return (`local.T1Score`) (`local.T2Score`)))

(fn `NewPlayer`
  (params (`Player State` :type "PlayerState Object Reference"))
  (bind _team1players (`self.Team1Players`))
  (bind _team2players (`self.Team2Players`))
  (if (> (`BlueprintSetLibrary.Set_Length` _team1players) (`BlueprintSetLibrary.Set_Length` _team2players))
    (`BlueprintSetLibrary.Set_Add` _team2players `Player State`)
    (bind _asfpsstate (cast `/Game/Player/FPSState` `Player State`))
    (set `/Game/Player/FPSState.TeamNumber` 2 _asfpsstate)
    (else
      (`BlueprintSetLibrary.Set_Add` _team1players `Player State`)
      (bind _asfpsstate_2 (cast `/Game/Player/FPSState` `Player State`))
      (set `/Game/Player/FPSState.TeamNumber` 1 _asfpsstate_2))))

(fn `RemovePlayer`
  (params (PlayerStateLeaving :type "PlayerState Object Reference"))
  (`BlueprintSetLibrary.Set_Remove` (`self.Team1Players`) PlayerStateLeaving)
  (`BlueprintSetLibrary.Set_Remove` (`self.Team2Players`) PlayerStateLeaving))

(fn `UserConstructionScript`
  (`parent.UserConstructionScript`))